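; BPBall is the game ball, launched from the player's paddle in what appears to be a Breakout-style game.
; On BeginPlay it disables physics on its sphere and caches the player paddle and BOGameMode.
; LaunchBall enables physics and applies a mass-independent X-axis impulse scaled by strength.
; When destroyed, it notifies the game mode through BallUsed.
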(event `self.ReceiveBeginPlay`
  ;[1 1 1] Set Player Paddle
  (`PrimitiveComponent.SetSimulatePhysics` (`self.Sphere`) false)
  (bind _asbppaddles (cast `/Game/Blueprints/BPPaddles` (`Controller.K2_GetPawn` (`GameplayStatics.GetPlayerController` 0))))
  (set `self.playerPaddle` _asbppaddles)
  ;[1 1 1] Get Game Mode
  (bind _asbogame_mode (cast `/Game/BOGameMode` (`GameplayStatics.GetGameMode`)))
  (set `self.gameMode` _asbogame_mode))

(event `LaunchBall`
  (params (Strength :type "Float (double-precision)"))
  ;[1 1 1] Launch Ball
  (`PrimitiveComponent.SetSimulatePhysics` (`self.Sphere`) true)
  (`PrimitiveComponent.AddImpulse` (`self.Sphere`) (`KismetMathLibrary.MakeVector` (* Strength (`self.fullStrength`))) "None" true))

(event `self.ReceiveDestroyed`
  ;[1 1 1] Spawn New Ball
  (`/Game/BOGameMode.BallUsed` (`self.gameMode`)))

(fn `UserConstructionScript`)