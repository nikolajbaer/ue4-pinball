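; BPPlayer is the player Blueprint for what appears to be a pinball game, turning input into launcher and paddle actions.
; LaunchBall press and release both call the Launcher with a released flag, and the NewBall event forwards to the Launcher to supply a ball.
; Left and right paddle inputs each drive two paddles through UsePaddle on press and release, always passing Clockwise as false.
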(event `NewBall`
  ;[1 1 1] New Ball
  (`/Game/Blueprints/BPLauncher.NewBall` (`self.launcher`)))

(event `InputAction|LaunchBall`
  (params (Key :type "Key Structure"))
  (bind _launcher (`self.launcher`))
  ;[1 1 1] Launch Ball
  (:`Pressed`
    (`/Game/Blueprints/BPLauncher.LaunchBall` _launcher false))
  (:`Released`
    (`/Game/Blueprints/BPLauncher.LaunchBall` _launcher true)))

(event `InputAction|LeftPaddle`
  (params (Key :type "Key Structure"))
  (bind _leftpaddle1 (`self.leftPaddle1`))
  (bind _leftpaddle2 (`self.leftPaddle2`))
  ;[1 1 1] Left Paddle
  (:`Pressed`
    (`/Game/Blueprints/BPPaddle.UsePaddle` _leftpaddle1 false false)
    (`/Game/Blueprints/BPPaddle.UsePaddle` _leftpaddle2 false false))
  (:`Released`
    (`/Game/Blueprints/BPPaddle.UsePaddle` _leftpaddle1 true false)
    (`/Game/Blueprints/BPPaddle.UsePaddle` _leftpaddle2 true false)))

(event `InputAction|RightPaddle`
  (params (Key :type "Key Structure"))
  (bind _rightpaddle1 (`self.rightPaddle1`))
  (bind _rightpaddle2 (`self.rightPaddle2`))
  ;[1 1 1] Right Paddle
  (:`Pressed`
    (`/Game/Blueprints/BPPaddle.UsePaddle` _rightpaddle1 false false)
    (`/Game/Blueprints/BPPaddle.UsePaddle` _rightpaddle2 false false))
  (:`Released`
    (`/Game/Blueprints/BPPaddle.UsePaddle` _rightpaddle1 true false)
    (`/Game/Blueprints/BPPaddle.UsePaddle` _rightpaddle2 true false)))

(fn `UserConstructionScript`)