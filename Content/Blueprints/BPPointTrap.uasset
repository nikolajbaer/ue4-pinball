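; BPPointTrap is a pinball trap that briefly holds a ball, launches it back out and awards points.
; On actor overlap with a BPBall, it disables physics simulation on the ball's sphere and zeroes its velocities.
; After a TrapTime delay, it re-enables physics and applies an ExitForce impulse along ExitArrow's forward vector.
; It then passes PointsOnTrap to BPPinballGameMode's UpdateScore.
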(event `self.ReceiveActorBeginOverlap`
  (params (OtherActor :type "Actor Object Reference"))
  ;[1 1 1] Capture and Release Ball
  (bind _asbpball (cast `/Game/Blueprints/BPBall` OtherActor))
  (bind _sphere (`/Game/Blueprints/BPBall.Sphere` _asbpball))
  (`PrimitiveComponent.SetSimulatePhysics` _sphere false)
  (`PrimitiveComponent.SetPhysicsLinearVelocity` _sphere (0.0 0.0 0.0) false "None")
  (`PrimitiveComponent.SetPhysicsAngularVelocityInDegrees` _sphere (0.0 0.0 0.0) false "None")
  (`KismetSystemLibrary.Delay` (`self.trapTime`))
  (`PrimitiveComponent.SetSimulatePhysics` _sphere true)
  (`PrimitiveComponent.AddImpulse` _sphere (* (`SceneComponent.GetForwardVector` (`self.ExitArrow`)) (`self.exitForce`)) "None" false)
  (bind _asbppinball_game_mode (cast `/Game/Blueprints/BPPinballGameMode` (`GameplayStatics.GetGameMode`)))
  (`/Game/Blueprints/BPPinballGameMode.UpdateScore` _asbppinball_game_mode (`self.pointsOnTrap`)))

(fn `UserConstructionScript`)