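; BPLauncher is the pinball ball launcher, spawning balls and firing them with a hold-to-charge shot.
; On BeginPlay it caches BPPinballGameMode and calls NewBall, which spawns a BPBall at the Arrow unless the game is over.
; LaunchBall records the press time, then on release fires any not-yet-active ball along the Arrow's forward vector.
; Launch strength scales with hold time over LaunchChargeTime, clamped to a minimum and maximum.
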(event `LaunchBall`
  (params (released :type Boolean))
  ;[1 1 1] LaunchBall
  (if released
    (if (not (`self.isBallActive`))
      (`/Game/Blueprints/BPBall.LaunchBall` (`self.activeBall`) (`KismetMathLibrary.FClamp` (* (- (`KismetSystemLibrary.GetGameTimeInSeconds`) (`self.launchStrengthStart`)) (/ 1.0 (`self.launchChargeTime`))) 0.25) (`SceneComponent.GetForwardVector` (`self.Arrow`)))
      (set `self.isBallActive` true))
    (else
      (set `self.launchStrengthStart` (`KismetSystemLibrary.GetGameTimeInSeconds`)))))

(event `self.ReceiveBeginPlay`
  ;[1 1 1] NewBall on BeginPlay
  (bind _asbppinball_game_mode (cast `/Game/Blueprints/BPPinballGameMode` (`GameplayStatics.GetGameMode`)))
  (set `self.gameMode` _asbppinball_game_mode)
  (`self.NewBall`))

(event `NewBall`
  ;[1 1 1] NewBall
  (if (not (`/Game/Blueprints/BPPinballGameMode.isGameOver` (`self.gameMode`)))
    (bind _returnvalue (`|SpawnActorFromClass` "/Game/Blueprints/BPBall.BPBall_C" (`SceneComponent.K2_GetComponentToWorld` (`self.Arrow`)) "Undefined" "OverrideRootScale" null null))
    (set `self.activeBall` _returnvalue)
    (set `self.isBallActive` false)))

(fn `UserConstructionScript`)